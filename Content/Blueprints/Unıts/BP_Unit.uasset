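; BP_Unit is a selectable unit that shows a Circle1 indicator while selected.
; It registers itself with player controller 0 on BeginPlay and unregisters on EndPlay, using message calls.
; Select and DeSelect events set the IsSelected flag and toggle the circle's visibility.
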(event EventBeginPlay
  (Class|BPIUnitRegistry|RegisterUnit(Message) (Game|GetPlayerController 0) self))

(event Collision|EventActorBeginOverlap
  (params (OtherActor :type Actor%20Object%20Reference)))

(event EventTick
  (params (DeltaSeconds :type Float%20%28single-precision%29)))

(event EventDeSelect
  (Variables|Default|SetbIsSelected false)
  (Rendering|SetVisibility (Variables|Default|GetCircle1) false false))

(event EventSelect
  (Variables|Default|SetbIsSelected true)
  (Rendering|SetVisibility (Variables|Default|GetCircle1) true false))

(event EventEndPlay
  (params (EndPlayReason :type EEndPlayReason%20Enum :default "Destroyed"))
  (Class|BPIUnitRegistry|UnregisterUnit(Message) (Game|GetPlayerController 0) self))

(fn ConstructionScript)